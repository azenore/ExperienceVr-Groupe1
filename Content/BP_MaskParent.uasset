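; Parent Blueprint for grabbable VR emotion masks that lerp back to their start transform when released.
; ActivateMask uses MaskIndex to set the BP_Eye iris, play sounds through spawned BP_Son actors and, for joy, sadness or boredom, stream a level.
; Those moods hide masks via the GameInstance, then timelines revert everything, destroy this mask and spawn BP_MaskEnd if none remain.
; The fear case instead triggers BP_ChaosAmphi destruction.
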(event OnGrabbed(GrabComponent)
  (Audio|PlaySound2D "/Game/Interface_Item_Sounds_LITE/MISC/cue/Prize_Count_1_1_Cue.Prize_Count_1_1_Cue" 1.0 1.0 0.0 0 0))

(event Custom|Activate%20Mask
  (bind _eye (Variables|Default|Geteye))
  (bind _as_bp_game_instance (Variables|Default|GetAs%20Bp%20Game%20Instance))
  (bind _mid_eye (Variables|/Game/Game/BP_Eye.BP_Eye_C|GetMID_Eye _eye))
  (Variables|Default|SetLazyFix true)
  (switch int (Variables|Default|GetMask%20Index)
    (:0
      (Rendering|Material|SetTextureParameterValue _mid_eye "Iris" "/Game/Game/TextPupilles/OeilJoie.OeilJoie")
      (Class|GameplayStatics|LoadStreamLevelbySoftObjectPtr "/Game/Levels/BLOCKINGVOLUME_AMPHI_JOIE.BLOCKINGVOLUME_AMPHI_JOIE" true false)
      (Utilities|AddSound "/Game/Game/Song/Music/S_JoySong.S_JoySong"
        (:Output
          (Utilities|AddSound "/Game/Game/Song/SoundEffects/serenitysoundeffect_Cue.serenitysoundeffect_Cue"
            (:Output
              (Utilities|AddSound "/Game/Game/Song/SoundEffects/SoundEffect_PlantsGrow3_Cue.SoundEffect_PlantsGrow3_Cue"
                (:Output
                  (Variables|/Game/Game/BLUEPRINTS/Bp_GameInstance.Bp_GameInstance_C|SetUsedMaskNb _as_bp_game_instance (+ (Variables|/Game/Game/BLUEPRINTS/Bp_GameInstance.Bp_GameInstance_C|GetUsedMaskNb _as_bp_game_instance) 1) :!label _label)
                  (Default|HideMasks (Variables|Default|GetAs%20Bp%20Game%20Instance))
                  (Utilities|FlowControl|Sequence
                    (:then_0
                      (bind _alpha (Timeline|Timeline Play)
                        (:Update
                          (Transformation|SetRelativeScale3D (Variables|/Game/Game/BP_Eye.BP_Eye_C|Geteyemesh (Variables|Default|Geteye)) (Math|Vector|MakeVector 1.0 _alpha _alpha)))
                        (:Finished
                          (Utilities|FlowControl|Sequence
                            (:then_0
                              (Audio|PlaySound2D "/Game/Interface_Item_Sounds_LITE/Interface/cue/Negative_14_2_Cue.Negative_14_2_Cue" 1.0 1.0 0.0 0 0)
                              (Rendering|Material|SetTextureParameterValue (Variables|/Game/Game/BP_Eye.BP_Eye_C|GetMID_Eye (Variables|Default|Geteye)) "Iris" "/Game/Game/TextPupilles/OeilBase.OeilBase")
                              (bind _alpha_2 (Timeline|Timeline_0 PlayFromStart)
                                (:Update
                                  (Transformation|SetRelativeScale3D (Variables|/Game/Game/BP_Eye.BP_Eye_C|Geteyemesh (Variables|Default|Geteye)) (Math|Vector|MakeVector 1.0 _alpha_2 _alpha_2)))
                                (:Finished
                                  (Actor|DestroyActor)
                                  (Variables|/Game/Game/BP_Mannequin.BP_Mannequin_C|SetHasMask (Variables|Default|GetMannequin) false)
                                  (Variables|/Game/VRTemplate/Blueprints/VRPawn.VRPawn_C|SetHasMask (Variables|Default|GetPlayer) false)
                                  (Default|CheckUsedMask (Variables|Default|GetAs%20Bp%20Game%20Instance))
                                  (bind _returnvalue (Actor|GetActorOfClass "BP_MaskParent_C"))
                                  (Utilities|IsValid _returnvalue
                                    (:Is%20Not%20Valid
                                      (Development|PrintString "THE END")
                                      (Game|SpawnActorfromClass "/Game/BP_MaskEnd.BP_MaskEnd_C" (Math|Transform|MakeTransform "421.612472,-11135.811479,355.492029" "0.000000,-89.000000,-89.000000" "1.000000,1.000000,1.000000") "Undefined" "MultiplyWithRoot" 0 0))))))
                            (:then_1
                              (Class|GameplayStatics|UnloadStreamLevelbySoftObjectPtr "/Game/Levels/BLOCKINGVOLUME_AMPHI_JOIE.BLOCKINGVOLUME_AMPHI_JOIE" false)
                              (for _array_element (Variables|Default|GetBP_SoundRef)
                                (Default|StopSound _array_element)))
                            (:then_2
                              (Class|GameplayStatics|UnloadStreamLevelbySoftObjectPtr "/Game/Levels/BLOCKINGVOLUME_AMPHI_SADNESS.BLOCKINGVOLUME_AMPHI_SADNESS" false))
                            (:then_3
                              (Class|GameplayStatics|UnloadStreamLevelbySoftObjectPtr "/Game/Levels/BlockingVolume_amphi_ennui.BlockingVolume_amphi_ennui" false))))))
                    (:then_1
                      (bind _alpha_3 (Timeline|Destroy PlayFromStart)
                        (:Update
                          (Transformation|SetRelativeScale3D (Variables|Default|GetStaticMesh) (Math|Vector|MakeVector _alpha_3 _alpha_3 _alpha_3)))))))))))))
    (:1
      (Rendering|Material|SetTextureParameterValue _mid_eye "Iris" "/Game/Game/TextPupilles/OeilMelancolie.OeilMelancolie")
      (Class|GameplayStatics|LoadStreamLevelbySoftObjectPtr "/Game/Levels/BLOCKINGVOLUME_AMPHI_SADNESS.BLOCKINGVOLUME_AMPHI_SADNESS" true false)
      (Utilities|AddSound "/Game/Game/Song/Music/sadsong_Cue.sadsong_Cue"
        (:Output
          (Utilities|AddSound "/Game/Game/Song/SoundEffects/sadsoundeffect_Cue.sadsoundeffect_Cue"
            (:Output
              (goto _label))))))
    (:2
      (Rendering|Material|SetTextureParameterValue _mid_eye "Iris" "/Game/Game/TextPupilles/OeilEnnuie.OeilEnnuie")
      (Class|GameplayStatics|LoadStreamLevelbySoftObjectPtr "/Game/Levels/BlockingVolume_amphi_ennui.BlockingVolume_amphi_ennui" true false)
      (Utilities|AddSound "/Game/Game/Song/Music/boredsong_Cue.boredsong_Cue"
        (:Output
          (Utilities|AddSound "/Game/Game/Song/SoundEffects/boredsoundeffect_Cue.boredsoundeffect_Cue"
            (:Output
              (Utilities|AddSound "/Game/Game/Song/SoundEffects/S_Sand.S_Sand"
                (:Output
                  (goto _label))))))))
    (:4
      (Utilities|AddSound "/Game/Game/Song/Music/fearsong_Cue.fearsong_Cue"
        (:Output
          (Rendering|Material|SetTextureParameterValue _mid_eye "Iris" "/Game/Game/TextPupilles/OeilFin.OeilFin")
          (bind _returnvalue_2 (Actor|GetActorOfClass "/Game/Game/ChaosDestruction/BP_ChaosAmphi.BP_ChaosAmphi_C"))
          (Default|Destruction _returnvalue_2)
          (bind _alpha_4 (Timeline|Timeline_1 PlayFromStart)
            (:Update
              (Transformation|SetRelativeScale3D (Variables|/Game/Game/BP_Eye.BP_Eye_C|Geteyemesh (Variables|Default|Geteye)) (Math|Vector|MakeVector 1.0 _alpha_4 _alpha_4)))))))))

(event Custom|HideMask
  (Rendering|SetVisibility (Variables|Default|GetStaticMesh) false false))

(event EventBeginPlay
  (bind _staticmesh (Variables|Default|GetStaticMesh))
  (bind _asbp_game_instance (Utilities|Casting|CastToBp_GameInstance (Game|GetGameInstance)))
  (bind _output_get (Variables|Default|SetAs%20Bp%20Game%20Instance _asbp_game_instance))
  (EventDispatchers|BindEventtoChangevisibleMask _output_get (delegate Custom|HideMask))
  (bind _returnvalue (Actor|GetActorOfClass "/Game/Game/BP_Eye.BP_Eye_C"))
  (Variables|Default|Seteye _returnvalue)
  (bind _returnvalue_2 (Actor|GetActorOfClass "/Game/Game/BP_Mannequin.BP_Mannequin_C"))
  (Variables|Default|SetMannequin _returnvalue_2)
  (Variables|Default|SetTargetLocation (Transformation|GetWorldLocation _staticmesh))
  (Variables|Default|SetTargetRotation (Transformation|GetWorldRotation _staticmesh))
  (bind _asvrpawn (Utilities|Casting|CastToVRPawn (Game|Player|GetPlayerPawn 0)))
  (Variables|Default|SetPlayer _asvrpawn))

(event Collision|EventActorBeginOverlap
  (params (OtherActor :type Actor%20Object%20Reference)))

(event EventTick
  (params (DeltaSeconds :type Float%20%28single-precision%29))
  (bind _returnvalue (* DeltaSeconds 5.0))
  (bind _staticmesh (Variables|Default|GetStaticMesh))
  (if (not (or (Variables|/Game/VRTemplate/Blueprints/GrabComponent.GrabComponent_C|GetbIsHeld (Variables|Default|GetGrabComponent)) (Variables|Default|GetLazyFix)))
    (Transformation|SetWorldLocationAndRotation (Variables|Default|GetStaticMesh) (Math|Vector|Lerp(Vector) (Transformation|GetWorldLocation _staticmesh) (Variables|Default|GetTargetLocation) _returnvalue) (Math|Rotator|Lerp(Rotator) (Transformation|GetWorldRotation _staticmesh) (Variables|Default|GetTargetRotation) _returnvalue) false false)))

(fn ConstructionScript)