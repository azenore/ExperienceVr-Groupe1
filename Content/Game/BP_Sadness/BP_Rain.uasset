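; Rain effect actor in BP_Sadness that fades its RainFx particle spawn rate in and out.
; On BeginPlay it binds StopRain to the Game Instance's stop-raining dispatcher, then ramps the spawn rate up from zero with the StartRainning timeline.
; StopRain ramps it back down through a second timeline and sets a finished flag, though the author's comment marks this fade-out as no longer used.
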(event Custom|StopRain
  ;[1 1 1] Animation Pluie s'arrête (Plus utilisé)
  (bind _appear (Timeline|Timeline Play)
    (:Update
      (Niagara|SetNiagaraVariable(Float) (Variables|Default|GetRain_fx) "SpawnRate" (Math|Float|Lerp 6e+02 0.0 _appear)))
    (:Finished
      (Variables|Default|SetStop%20Rain true))))

(event EventBeginPlay
  ;[1 1 1] Récupère et met dans une varaiable la Game Instance
  (bind _asbp_game_instance (Utilities|Casting|CastToBp_GameInstance (Game|GetGameInstance)))
  (bind _output_get (Variables|Default|SetAs%20Bp%20Game%20Instance _asbp_game_instance))
  (EventDispatchers|BindEventtoStopRainning _output_get (delegate Custom|StopRain))
  ;[1 1 1] Animation pluie commence
  (Niagara|SetNiagaraVariable(Float) (Variables|Default|GetRain_fx) "SpawnRate" 0.0)
  (bind _appear (Timeline|StartRainning Play)
    (:Update
      (Niagara|SetNiagaraVariable(Float) (Variables|Default|GetRain_fx) "SpawnRate" (Math|Float|Lerp 0.0 6e+02 _appear)))))

(event Collision|EventActorBeginOverlap
  (params (OtherActor :type Actor%20Object%20Reference)))

(event EventTick
  (params (DeltaSeconds :type Float%20%28single-precision%29)))

(fn ConstructionScript)