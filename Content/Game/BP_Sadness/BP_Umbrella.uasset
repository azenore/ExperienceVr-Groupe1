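; BP_Umbrella is a grabbable umbrella actor that drifts back to its starting position and rotation whenever it is not held.
; BeginPlay caches the game instance and, if that cast succeeds, records the root's world location and rotation as the return target.
; While GrabComponent reports not held, Tick lerps the root toward that target using an alpha scaled by DeltaSeconds, giving an eased return.
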(event EventBeginPlay
  (bind _defaultsceneroot (Variables|Default|GetDefaultSceneRoot))
  (bind _asbp_game_instance (Utilities|Casting|CastToBp_GameInstance (Game|GetGameInstance)))
  (Variables|Default|SetAs%20Bp%20Game%20Instance _asbp_game_instance)
  (Variables|Default|SetTargetRotation (Transformation|GetWorldRotation _defaultsceneroot))
  (Variables|Default|SetTargetLocat (Transformation|GetWorldLocation _defaultsceneroot)))

(event Collision|EventActorBeginOverlap
  (params (OtherActor :type Actor%20Object%20Reference)))

(event EventTick
  (params (DeltaSeconds :type Float%20%28single-precision%29))
  (bind _returnvalue (* DeltaSeconds 5.0))
  (bind _defaultsceneroot (Variables|Default|GetDefaultSceneRoot))
  ;[1 1 1] Ramène Le parapluie à sa position initiale
  (if (not (Variables|/Game/VRTemplate/Blueprints/GrabComponent.GrabComponent_C|GetbIsHeld (Variables|Default|GetGrabComponent)))
    (Transformation|SetWorldLocationAndRotation (Variables|Default|GetDefaultSceneRoot) (Math|Vector|Lerp(Vector) (Transformation|GetWorldLocation _defaultsceneroot) (Variables|Default|GetTargetLocat) _returnvalue) (Math|Rotator|Lerp(Rotator) (Transformation|GetWorldRotation _defaultsceneroot) (Variables|Default|GetTargetRotation) _returnvalue) false false)))

(fn ConstructionScript)