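; BP_Cigale is an actor whose sphere travels along the level's BP_Spline at a time-based speed.
; BeginPlay fades out a black screen, then starts movement after a ten-second delay.
; Tick converts time elapsed since departure into spline distance, looping by modulo except in FinalMap.
; There, reaching the spline's end triggers a fade-in and loads VRTemplateMap.
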(event Custom|EndTransition
  (Default|Fadein (Variables|Default|GetBlackScreen))
  (Utilities|FlowControl|Delay 1.1)
  (Game|OpenLevel(byName) "VRTemplateMap"))

(event EventBeginPlay
  (bind _returnvalue (Actor|GetActorOfClass "/Game/Game/Yoann/BP_Spline.BP_Spline_C"))
  (Variables|Default|SetBP_Spline _returnvalue)
  (bind _returnvalue_2 (UserInterface|CreateWidget "/Game/Game/Yoann/BPW_BlackScreen.BPW_BlackScreen_C"))
  (bind _output_get (Variables|Default|SetBlackScreen _returnvalue_2))
  (Default|FadeOut _output_get)
  (bind _returnvalue_3 (Game|GetCurrentLevelName true))
  (Variables|Default|SetLevelName _returnvalue_3)
  (Utilities|FlowControl|Delay 1e+01)
  (Variables|Default|SetIsMoving true))

(event EventTick
  (params (DeltaSeconds :type Float%20%28single-precision%29))
  (bind _bp_spline (Variables|Default|GetBP_Spline))
  (bind _bp_spline_2 (Variables|Default|GetBP_Spline))
  (bind _spline (Variables|/Game/Game/Yoann/BP_Spline.BP_Spline_C|GetSpline _bp_spline))
  (bind _spline_2 (Variables|/Game/Game/Yoann/BP_Spline.BP_Spline_C|GetSpline _bp_spline_2))
  (if (Variables|Default|GetIsMoving)
    (if (Utilities|Enum|Equal(Enum) (Variables|Default|GetLevelName) "FinalMap")
      (if (<= (Spline|GetSplineLength _spline) (* (- (Utilities|Time|GetTimeSeconds) (Variables|Default|GetConteurTemps)) (Variables|Default|GetSpeed)))
        (CallFunction|EndTransition)
        (else
          (Transformation|SetWorldLocation (Variables|Default|GetSphere) (Spline|GetLocationatDistanceAlongSpline _spline (* (- (Utilities|Time|GetTimeSeconds) (Variables|Default|GetConteurTemps)) (Variables|Default|GetSpeed)) "World") false false)))
      (else
        (Transformation|SetWorldLocation (Variables|Default|GetSphere) (Spline|GetLocationatDistanceAlongSpline _spline_2 (Math|Float|%(Float) (* (- (Utilities|Time|GetTimeSeconds) (Variables|Default|GetConteurTemps)) (Variables|Default|GetSpeed)) (Spline|GetSplineLength _spline_2)) "World") false false)))
    (else
      (Variables|Default|SetConteurTemps (Utilities|Time|GetTimeSeconds)))))

(fn ConstructionScript)

(fn Deplacement)