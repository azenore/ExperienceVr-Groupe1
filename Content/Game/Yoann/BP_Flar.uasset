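; BP_Flar is an actor whose sphere travels in a loop along a BP_Spline path while IsMoving is set and the game has not ended.
; Each Tick derives spline distance from elapsed time since ConteurTemps times Speed, wrapped by spline length, and triggers two shine sounds every frame.
; Without a valid spline, it waits a second, then finds one in the level.
; The Deplacement function is empty.
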(event EventBeginPlay
  (bind _asbp_game_instance (Utilities|Casting|CastToBp_GameInstance (Game|GetGameInstance))))

(event EventTick
  (params (DeltaSeconds :type Float%20%28single-precision%29))
  (if (not (Variables|/Game/Game/BLUEPRINTS/Bp_GameInstance.Bp_GameInstance_C|GetTheEnd (stale EventBeginPlay _asbp_game_instance)))
    (if (Variables|Default|GetIsMoving)
      (bind _bp_spline (Variables|Default|GetBP_Spline)
        (:then
          (Transformation|SetWorldLocation (Variables|Default|GetSphere) (Spline|GetLocationatDistanceAlongSpline (Variables|/Game/Game/Yoann/BP_Spline.BP_Spline_C|GetSpline _bp_spline) (Math|Float|%(Float) (* (- (Utilities|Time|GetTimeSeconds) (Variables|Default|GetConteurTemps)) (Variables|Default|GetSpeed)) (Spline|GetSplineLength (Variables|/Game/Game/Yoann/BP_Spline.BP_Spline_C|GetSpline _bp_spline))) "World") false false)
          (Audio|PlaySound2D "/Game/Game/Song/SoundEffects/shine-1-268902_Cue.shine-1-268902_Cue" 1.0 1.0 0.0 0 0)
          (Audio|PlaySound2D "/Game/Game/Song/SoundEffects/shimmering-object-79354_Cue.shimmering-object-79354_Cue" 1.0 1.0 0.0 0 0))
        (:else
          (Utilities|FlowControl|Delay 1.0)
          (Variables|Default|GetBP_Spline
            (:then)
            (:else
              (bind _returnvalue (Actor|GetActorOfClass "/Game/Game/Yoann/BP_Spline.BP_Spline_C"))
              (Variables|Default|SetBP_Spline _returnvalue))))))))

(fn ConstructionScript)

(fn Deplacement)