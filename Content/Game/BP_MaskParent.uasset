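; Base mask actor, a grabbable mesh that eases back to its starting transform whenever it is not held, until activated.
; ActivateMask streams in a level by MaskIndex (joy or sadness amphi blocking volumes; third case has none set) while shrinking the mask.
; Two chained timelines animate BP_Eye's mesh scale; between them both levels unload.
; Afterwards the actor destroys itself and clears the mannequin's HasMask flag.
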(event Custom|Activate%20Mask
  (Variables|Default|SetLazyFix true)
  (switch int (Variables|Default|GetMask%20Index)
    (:0
      (Class|GameplayStatics|LoadStreamLevelbySoftObjectPtr "/Game/Levels/BLOCKINGVOLUME_AMPHI_JOIE.BLOCKINGVOLUME_AMPHI_JOIE" true false))
    (:1
      (Class|GameplayStatics|LoadStreamLevelbySoftObjectPtr "/Game/Levels/BLOCKINGVOLUME_AMPHI_SADNESS.BLOCKINGVOLUME_AMPHI_SADNESS" true false))
    (:2
      (Class|GameplayStatics|LoadStreamLevelbySoftObjectPtr 0 false false)))
  (Utilities|FlowControl|Sequence
    (:then_0
      (bind _alpha (Timeline|Timeline PlayFromStart)
        (:Update
          (Transformation|SetRelativeScale3D (Variables|/Game/Game/BP_Eye.BP_Eye_C|Geteyemesh (Variables|Default|Geteye)) (Math|Vector|MakeVector 1.0 _alpha _alpha)))
        (:Finished
          (Utilities|FlowControl|Sequence
            (:then_0
              (bind _alpha_2 (Timeline|Timeline_0 PlayFromStart)
                (:Update
                  (Transformation|SetRelativeScale3D (Variables|/Game/Game/BP_Eye.BP_Eye_C|Geteyemesh (Variables|Default|Geteye)) (Math|Vector|MakeVector 1.0 _alpha_2 _alpha_2)))
                (:Finished
                  (Actor|DestroyActor)
                  (Variables|/Game/Game/BP_Mannequin.BP_Mannequin_C|SetHasMask (Variables|Default|GetMannequin) false))))
            (:then_1
              (Class|GameplayStatics|UnloadStreamLevelbySoftObjectPtr "/Game/Levels/BLOCKINGVOLUME_AMPHI_JOIE.BLOCKINGVOLUME_AMPHI_JOIE" false))
            (:then_2
              (Class|GameplayStatics|UnloadStreamLevelbySoftObjectPtr "/Game/Levels/BLOCKINGVOLUME_AMPHI_SADNESS.BLOCKINGVOLUME_AMPHI_SADNESS" false))))))
    (:then_1
      (bind _alpha_3 (Timeline|Destroy PlayFromStart)
        (:Update
          (Transformation|SetRelativeScale3D (Variables|Default|GetStaticMesh) (Math|Vector|MakeVector _alpha_3 _alpha_3 _alpha_3)))))))

(event EventBeginPlay
  (bind _staticmesh (Variables|Default|GetStaticMesh))
  (bind _returnvalue (Actor|GetActorOfClass "/Game/Game/BP_Eye.BP_Eye_C"))
  (Variables|Default|Seteye _returnvalue)
  (bind _returnvalue_2 (Actor|GetActorOfClass "/Game/Game/BP_Mannequin.BP_Mannequin_C"))
  (Variables|Default|SetMannequin _returnvalue_2)
  (Variables|Default|SetTargetLocation (Transformation|GetWorldLocation _staticmesh))
  (Variables|Default|SetTargetRotation (Transformation|GetWorldRotation _staticmesh)))

(event Collision|EventActorBeginOverlap
  (params (OtherActor :type Actor%20Object%20Reference)))

(event EventTick
  (params (DeltaSeconds :type Float%20%28single-precision%29))
  (bind _returnvalue (* DeltaSeconds 5.0))
  (bind _staticmesh (Variables|Default|GetStaticMesh))
  (if (not (or (Variables|/Game/VRTemplate/Blueprints/GrabComponent.GrabComponent_C|GetbIsHeld (Variables|Default|GetGrabComponent)) (Variables|Default|GetLazyFix)))
    (Transformation|SetWorldLocationAndRotation (Variables|Default|GetStaticMesh) (Math|Vector|Lerp(Vector) (Transformation|GetWorldLocation _staticmesh) (Variables|Default|GetTargetLocation) _returnvalue) (Math|Rotator|Lerp(Rotator) (Transformation|GetWorldRotation _staticmesh) (Variables|Default|GetTargetRotation) _returnvalue) false false)))

(fn ConstructionScript)