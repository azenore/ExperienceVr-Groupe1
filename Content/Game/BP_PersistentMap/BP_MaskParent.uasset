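; Base VR grabbable mask that, on activation, turns the amphitheatre into an emotional scene (joy, melancholy, boredom, surprise) or the ending, then glides home when released unused.
; MaskIndex picks the colour, eye iris, streamed level and sounds, while Game Instance events hide and restore masks.
; Timelines drive MPC colours, eye closing and cleanup.
; The last mask used spawns BP_MaskEnd; the ending fades out and reopens the default map.
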(event OnGrabbed(GrabComponent)
  ;[1 1 1] Son quand masque attrapé
  (Audio|PlaySound2D "/Game/Interface_Item_Sounds_LITE/MISC/cue/Prize_Count_1_1_Cue.Prize_Count_1_1_Cue" 1.0 1.0 0.0 0 0))

(event Custom|Activate%20Mask
  (bind _eye (Variables|Default|Geteye))
  (bind _as_bp_game_instance (Variables|Default|GetAs%20Bp%20Game%20Instance))
  (bind _as_bp_game_instance_2 (Variables|Default|GetAs%20Bp%20Game%20Instance))
  (bind _mid_eye (Variables|/Game/Game/BP_PersistentMap/BP_Eye.BP_Eye_C|GetMID_Eye _eye))
  (Variables|Default|SetBrightness 1.0)
  (Variables|Default|SetColor "(R=1.000000,G=1.000000,B=1.000000,A=1.000000)")
  (Variables|Default|SetMaskInUse true)
  ;[1 1 1] En fonction du masque activé :
  (switch int (Variables|Default|GetMask%20Index)
    (:0
      ;;[1 1 1] Changement couleur Amphi
      ;;;[1 1 1] Couleur Joie
      (Variables|Default|SetBrightness 1.0)
      (Variables|Default|SetColor "(R=0.564712,G=0.871367,B=0.412543,A=1.000000)")
      ;;[1 1 1] Changement Pupille Oeil
      (Rendering|Material|SetTextureParameterValue _mid_eye "Iris" "/Game/Game/TextPupils/OeilJoie.OeilJoie")
      ;;[1 1 1] Charge le niveau adapté
      (Class|GameplayStatics|LoadStreamLevelbySoftObjectPtr "/Game/Levels/BLOCKINGVOLUME_AMPHI_JOIE.BLOCKINGVOLUME_AMPHI_JOIE" true false)
      ;;[1 1 1] Ajoute les sons
      (Utilities|AddSound "/Game/Game/Sound/Music/S_JoySong.S_JoySong"
        (:Output
          (Utilities|AddSound "/Game/Game/Sound/SoundEffects/serenitysoundeffect_Cue.serenitysoundeffect_Cue"
            (:Output
              (Utilities|AddSound "/Game/Game/Sound/SoundEffects/SoundEffect_PlantsGrow3_Cue.SoundEffect_PlantsGrow3_Cue"
                (:Output
                  ;;[1 1 1] Compteur de masques utilisés
                  (Variables|/Game/Game/BLUEPRINTS/Bp_GameInstance.Bp_GameInstance_C|SetUsedMaskNb _as_bp_game_instance_2 (+ (Variables|/Game/Game/BLUEPRINTS/Bp_GameInstance.Bp_GameInstance_C|GetUsedMaskNb _as_bp_game_instance_2) 1) :!label _label)
                  ;[1 1 1] Passe par la game instance pour cacher les autres masques
                  (Default|HideMasks _as_bp_game_instance)
                  (Variables|/Game/Game/BLUEPRINTS/Bp_GameInstance.Bp_GameInstance_C|SetHideMask _as_bp_game_instance true)
                  (Utilities|FlowControl|Sequence
                    (:then_0
                      ;[1 1 1] Ferme L'oeil
                      (bind _alpha (Timeline|Ferme%20l'oeil PlayFromStart)
                        (:Update
                          (Transformation|SetRelativeScale3D (Variables|/Game/Game/BP_PersistentMap/BP_Eye.BP_Eye_C|Geteyemesh (Variables|Default|Geteye)) (Math|Vector|MakeVector 1.0 _alpha _alpha)))
                        (:Finished
                          (Utilities|FlowControl|Sequence
                            (:then_0
                              (Audio|PlaySound2D "/Game/Interface_Item_Sounds_LITE/Interface/cue/Negative_14_2_Cue.Negative_14_2_Cue" 1.0 1.0 0.0 0 0)
                              ;[1 1 1] Remet la pupille de Base
                              (Rendering|Material|SetTextureParameterValue (Variables|/Game/Game/BP_PersistentMap/BP_Eye.BP_Eye_C|GetMID_Eye (Variables|Default|Geteye)) "Iris" "/Game/Game/TextPupils/OeilBase.OeilBase")
                              ;[1 1 1] Réouvre l'oeil
                              (bind _alpha_2 (Timeline|Ouvre%20l'oeil PlayFromStart)
                                (:Update
                                  (Transformation|SetRelativeScale3D (Variables|/Game/Game/BP_PersistentMap/BP_Eye.BP_Eye_C|Geteyemesh (Variables|Default|Geteye)) (Math|Vector|MakeVector 1.0 _alpha_2 _alpha_2))
                                  ;[1 1 1] Remet l'amphi aux couleurs de Base
                                  (Rendering|Material|SetScalarParameterValue "/Game/Game/MPC/MPC_Colliseum.MPC_Colliseum" "Brightness" (Math|Float|Lerp (Variables|Default|GetBrightness) 1.0 _alpha_2) :!class /Script/Engine.KismetMaterialLibrary)
                                  (Rendering|Material|SetVectorParameterValue "/Game/Game/MPC/MPC_Colliseum.MPC_Colliseum" "Color" (Math|Color|Lerp(LinearColor) (Variables|Default|GetColor) "(R=1.000000,G=1.000000,B=1.000000,A=1.000000)" _alpha_2) :!class /Script/Engine.KismetMaterialLibrary))
                                (:Finished
                                  (Actor|DestroyActor)
                                  (Variables|/Game/Game/BP_PersistentMap/BP_Mannequin.BP_Mannequin_C|SetHasMask (Variables|Default|GetMannequin) false)
                                  (Variables|/Game/VRTemplate/Blueprints/VRPawn.VRPawn_C|SetHasMask (Variables|Default|GetPlayer) false)
                                  ;[1 1 1] Test Si tout les maques ont été utlisés, si oui, fait apparaître le masque de Fin
                                  (bind _returnvalue (Actor|GetActorOfClass "BP_MaskParent_C"))
                                  (Utilities|IsValid _returnvalue
                                    (:Is%20Not%20Valid
                                      (Game|SpawnActorfromClass "/Game/Game/BP_PersistentMap/BP_MaskEnd.BP_MaskEnd_C" (Math|Transform|MakeTransform "454.678730,-11101.928608,350.943188" "0.000000,-89.000000,-89.000000" "1.000000,1.000000,1.000000") "Undefined" "MultiplyWithRoot" 0 0))))))
                            (:then_1
                              ;[1 1 1] Décharge le niveau
                              (Class|GameplayStatics|UnloadStreamLevelbySoftObjectPtr "/Game/Levels/BLOCKINGVOLUME_AMPHI_JOIE.BLOCKINGVOLUME_AMPHI_JOIE" false)
                              ;[1 1 1] Arrête tout les sons
                              (for _array_element (Variables|Default|GetBP_SoundRef)
                                (Default|StopSound _array_element))
                              ;[1 1 1] Utilise la game instance pour rendre visible les masques restants
                              (Default|Showmask (Variables|Default|GetAs%20Bp%20Game%20Instance)))
                            (:then_2
                              (Class|GameplayStatics|UnloadStreamLevelbySoftObjectPtr "/Game/Levels/BLOCKINGVOLUME_AMPHI_SADNESS.BLOCKINGVOLUME_AMPHI_SADNESS" false))
                            (:then_3
                              (Class|GameplayStatics|UnloadStreamLevelbySoftObjectPtr "/Game/Levels/BlockingVolume_amphi_ennui.BlockingVolume_amphi_ennui" false))
                            (:then_4
                              (Class|GameplayStatics|UnloadStreamLevelbySoftObjectPtr "/Game/Levels/BLOKINGVOLUME_Surprise.BLOKINGVOLUME_Surprise" false))))))
                    (:then_1
                      ;[1 1 1] Détruit le Masque Utilisé
                      (bind _alpha_3 (Timeline|Destroy PlayFromStart)
                        (:Update
                          (Transformation|SetRelativeScale3D (Variables|Default|GetStaticMesh) (Math|Vector|MakeVector _alpha_3 _alpha_3 _alpha_3))
                          (Rendering|Material|SetScalarParameterValue "/Game/Game/MPC/MPC_Colliseum.MPC_Colliseum" "Brightness" (Math|Float|Lerp (Variables|Default|GetBrightness) 1.0 (* _alpha_3 4.0)) :!class /Script/Engine.KismetMaterialLibrary)
                          (Rendering|Material|SetVectorParameterValue "/Game/Game/MPC/MPC_Colliseum.MPC_Colliseum" "Color" (Math|Color|Lerp(LinearColor) (Variables|Default|GetColor) "(R=1.000000,G=1.000000,B=1.000000,A=1.000000)" (* _alpha_3 4.0)) :!class /Script/Engine.KismetMaterialLibrary))))))))))))
    (:1
      ;;;[1 1 1] Couleur Melancolie
      (Variables|Default|SetBrightness 1.0)
      (Variables|Default|SetColor "(R=0.391573,G=0.651406,B=0.768151,A=1.000000)")
      (Rendering|Material|SetTextureParameterValue _mid_eye "Iris" "/Game/Game/TextPupils/OeilMelancolie.OeilMelancolie")
      (Class|GameplayStatics|LoadStreamLevelbySoftObjectPtr "/Game/Levels/BLOCKINGVOLUME_AMPHI_SADNESS.BLOCKINGVOLUME_AMPHI_SADNESS" true false)
      (Utilities|AddSound "/Game/Game/Sound/Music/sadsong_Cue.sadsong_Cue"
        (:Output
          (Utilities|AddSound "/Game/Game/Sound/SoundEffects/sadsoundeffect_Cue.sadsoundeffect_Cue"
            (:Output
              (goto _label))))))
    (:2
      ;;;[1 1 1] Couleur Ennuie
      (Variables|Default|SetBrightness 1.0)
      (Variables|Default|SetColor "(R=1.000000,G=0.568627,B=0.325490,A=1.000000)")
      (Rendering|Material|SetTextureParameterValue _mid_eye "Iris" "/Game/Game/TextPupils/OeilEnnuie.OeilEnnuie")
      (Class|GameplayStatics|LoadStreamLevelbySoftObjectPtr "/Game/Levels/BlockingVolume_amphi_ennui.BlockingVolume_amphi_ennui" true false)
      (Utilities|AddSound "/Game/Game/Sound/Music/boredsong_Cue.boredsong_Cue"
        (:Output
          (Utilities|AddSound "/Game/Game/Sound/SoundEffects/boredsoundeffect_Cue.boredsoundeffect_Cue"
            (:Output
              (Utilities|AddSound "/Game/Game/Sound/SoundEffects/S_Sand.S_Sand"
                (:Output
                  (goto _label))))))))
    (:3
      ;;;[1 1 1] Couleur Surprise
      (Variables|Default|SetBrightness 1.0)
      (Variables|Default|SetColor "(R=1.000000,G=0.513726,B=0.847059,A=1.000000)")
      (Rendering|Material|SetTextureParameterValue _mid_eye "Iris" "/Game/Game/TextPupils/OeilSurprise.OeilSurprise")
      (Class|GameplayStatics|LoadStreamLevelbySoftObjectPtr "/Game/Levels/BLOKINGVOLUME_Surprise.BLOKINGVOLUME_Surprise" true false)
      (Utilities|AddSound "/Game/Game/Sound/Music/S_SurpriseMusic.S_SurpriseMusic"
        (:Output
          (Utilities|AddSound "/Game/Game/Sound/SoundEffects/S_Fireworks.S_Fireworks"
            (:Output
              (goto _label))))))
    (:4
      ;[1 1 1] Masque FIN
      (Variables|/Game/Game/BLUEPRINTS/Bp_GameInstance.Bp_GameInstance_C|SetTheEnd (Variables|Default|GetAs%20Bp%20Game%20Instance) true)
      (Class|GameplayStatics|LoadStreamLevelbySoftObjectPtr "/Game/Levels/BLOKINGVOLUME_FIN.BLOKINGVOLUME_FIN" true false)
      (Utilities|AddSound "/Game/Game/Sound/Music/FearSong2_Cue.FearSong2_Cue"
        (:Output
          (Rendering|Material|SetTextureParameterValue _mid_eye "Iris" "/Game/Game/TextPupils/OeilFin.OeilFin")
          (Transformation|SetRelativeScale3D (Variables|/Game/Game/BP_PersistentMap/BP_Eye.BP_Eye_C|Geteyemesh (Variables|Default|Geteye)) (Math|Vector|MakeVector 1.0 0.5 0.5))
          (Utilities|FlowControl|Sequence
            (:then_0
              (Timeline|Destroy PlayFromStart))
            (:then_1
              (Utilities|FlowControl|Delay 15.0)
              ;;[1 1 1] Crée un Dégradé Noir sur la vision du joeur
              (bind _alpha_4 (Timeline|Fade Play)
                (:Update
                  (Rendering|Material|SetScalarParameterValue "/Game/Game/MPC/MPC_Fade.MPC_Fade" "Opacity" _alpha_4 :!class /Script/Engine.KismetMaterialLibrary))
                (:Finished
                  ;;[1 1 1] Reset le jeu pour le prochain joueur
                  (Utilities|FlowControl|Delay 1.0)
                  (Audio|PlaySound2D "/Game/Game/Sound/SoundEffects/S_EndEffect.S_EndEffect" 1.0 1.0 0.0 0 0)
                  (Utilities|FlowControl|Delay 1e+01)
                  (Game|OpenLevel(byObjectReference) "/Game/Levels/DEFAULT_MAP.DEFAULT_MAP"))))))))))

(event Custom|ShowMask
  ;[1 1 1] Quand On fini un "niveau" les masques restant sont à nouveau visible
  (Rendering|SetVisibility (Variables|Default|GetStaticMesh) true false))

(event Custom|HideMask
  ;[1 1 1] Quand On utilise un masque les autres sont invisible
  (if (not (== (Variables|/Game/VRTemplate/Blueprints/GrabComponent.GrabComponent_C|GetGrabType (Variables|Default|GetGrabComponent)) 0))
    (Rendering|SetVisibility (Variables|Default|GetStaticMesh) false false)))

(event Custom|stop%20Rain
  ;[1 1 1] Arrete le son de la pluie uniquement
  (Default|StopSound (Utilities|Array|Get(acopy) (Variables|Default|GetBP_SoundRef) 1)))

(event EventBeginPlay
  (bind _staticmesh (Variables|Default|GetStaticMesh))
  ;[1 1 1] Permet de communiquer avec la Game Instance
  (bind _asbp_game_instance (Utilities|Casting|CastToBp_GameInstance (Game|GetGameInstance)))
  (bind _output_get (Variables|Default|SetAs%20Bp%20Game%20Instance _asbp_game_instance))
  ;[1 1 1] Quand On utilise un masque les autres sont invisible
  (EventDispatchers|BindEventtoChangevisibleMask _output_get (delegate Custom|HideMask))
  ;[1 1 1] Quand On fini un "niveau" les masques restant sont à nouveau visible
  (EventDispatchers|BindEventtoVisibleMask _output_get (delegate Custom|ShowMask))
  ;[1 1 1] Arrete le son de la pluie uniquement
  (EventDispatchers|BindEventtoStopRainning _output_get (delegate Custom|stop%20Rain))
  ;[1 1 1] Récupère et place en variable le mannequin et l'oeil
  (bind _returnvalue (Actor|GetActorOfClass "/Game/Game/BP_PersistentMap/BP_Eye.BP_Eye_C"))
  (Variables|Default|Seteye _returnvalue)
  (bind _returnvalue_2 (Actor|GetActorOfClass "/Game/Game/BP_PersistentMap/BP_Mannequin.BP_Mannequin_C"))
  (Variables|Default|SetMannequin _returnvalue_2)
  ;[1 1 1] Récupère et place en variable la position et rotation initiale du masque
  (Variables|Default|SetTargetLocation (Transformation|GetWorldLocation _staticmesh))
  (Variables|Default|SetTargetRotation (Transformation|GetWorldRotation _staticmesh))
  ;[1 1 1] Récupère et place en variable le VrPawn (Le joueur)
  (bind _asvrpawn (Utilities|Casting|CastToVRPawn (Game|Player|GetPlayerPawn 0)))
  (Variables|Default|SetPlayer _asvrpawn))

(event EventTick
  (params (DeltaSeconds :type Float%20%28single-precision%29))
  (bind _returnvalue (* DeltaSeconds 5.0))
  (bind _staticmesh (Variables|Default|GetStaticMesh))
  ;[1 1 1] Repositionnement du masque sur la table si laché
  (if (not (or (Variables|/Game/VRTemplate/Blueprints/GrabComponent.GrabComponent_C|GetbIsHeld (Variables|Default|GetGrabComponent)) (Variables|Default|GetMaskInUse)))
    (Transformation|SetWorldLocationAndRotation (Variables|Default|GetStaticMesh) (Math|Vector|Lerp(Vector) (Transformation|GetWorldLocation _staticmesh) (Variables|Default|GetTargetLocation) _returnvalue) (Math|Rotator|Lerp(Rotator) (Transformation|GetWorldRotation _staticmesh) (Variables|Default|GetTargetRotation) _returnvalue) false false)))

(fn ConstructionScript)