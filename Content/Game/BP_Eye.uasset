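; BP_Eye is an eye actor with lash meshes that tracks the VR player's camera.
; Each tick it re-orients along the camera-to-eye line and repositions itself one unit from the eye mesh.
; It also eases the shared MPC_Eye PlayerLocation parameter toward the camera for smoothed material-side tracking.
; Construction positions the eye mesh and matches lash scale to the actor; the dynamic material's Iris texture setter is unconnected.
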(event EventTick
  (params (DeltaSeconds :type Float%20%28single-precision%29))
  (bind _returnvalue (Transformation|GetActorUpVector))
  (bind _player (Variables|Default|GetPlayer))
  (bind _eyemesh (Variables|Default|Geteyemesh))
  (bind _returnvalue_2 (Transformation|GetWorldLocation _eyemesh))
  (bind _camera (Variables|/Game/VRTemplate/Blueprints/VRPawn.VRPawn_C|GetCamera _player))
  (bind _returnvalue_3 (Transformation|GetWorldLocation _camera))
  (bind _returnvalue_4 (- _returnvalue_2 _returnvalue_3))
  (bind _returnvalue_5 (Math|Vector|Normalize _returnvalue_4))
  (bind _returnvalue_6 (Math|Rotator|MakeRotfromXZ _returnvalue_5 _returnvalue))
  (Transformation|SetActorLocation (+ _returnvalue_2 (Math|Vector|GetUpVector _returnvalue_6)) false false)
  (Transformation|SetActorRotation _returnvalue_6)
  (bind _returnvalue_7 (Rendering|Material|GetVectorParameterValue "/Game/Game/MPC_Eye.MPC_Eye" "PlayerLocation" :!class /Script/Engine.KismetMaterialLibrary))
  (Rendering|Material|SetVectorParameterValue "/Game/Game/MPC_Eye.MPC_Eye" "PlayerLocation" (Utilities|Struct|MakeLinearColor (.x (Math|Vector|Lerp(Vector) (Math|Vector|MakeVector (.r _returnvalue_7) (.g _returnvalue_7) (.b _returnvalue_7)) (Transformation|GetWorldLocation (Variables|/Game/VRTemplate/Blueprints/VRPawn.VRPawn_C|GetCamera (Variables|Default|GetPlayer))) (* DeltaSeconds 2.5))) (.y (Math|Vector|Lerp(Vector) (Math|Vector|MakeVector (.r _returnvalue_7) (.g _returnvalue_7) (.b _returnvalue_7)) (Transformation|GetWorldLocation (Variables|/Game/VRTemplate/Blueprints/VRPawn.VRPawn_C|GetCamera (Variables|Default|GetPlayer))) (* DeltaSeconds 2.5))) (.z (Math|Vector|Lerp(Vector) (Math|Vector|MakeVector (.r _returnvalue_7) (.g _returnvalue_7) (.b _returnvalue_7)) (Transformation|GetWorldLocation (Variables|/Game/VRTemplate/Blueprints/VRPawn.VRPawn_C|GetCamera (Variables|Default|GetPlayer))) (* DeltaSeconds 2.5))) 1.0) :!class /Script/Engine.KismetMaterialLibrary))

(event EventBeginPlay
  (bind _asvrpawn (Utilities|Casting|CastToVRPawn (Game|Player|GetPlayerPawn 0)))
  (Variables|Default|SetPlayer _asvrpawn)
  (bind _returnvalue (Rendering|Material|CreateDynamicMaterialInstance (Variables|Default|Geteyemesh) 0 "/Game/Game/MI_Eye.MI_Eye" "None" :!class /Script/Engine.PrimitiveComponent))
  (Variables|Default|SetMID_Eye _returnvalue))

(fn ConstructionScript
  (Transformation|SetRelativeLocationAndRotation (Variables|Default|Geteyemesh) (- (Transformation|GetActorLocation) "0.000000,0.000000,1.000000") (Transformation|GetActorRotation) false false)
  (Transformation|SetWorldScale3D (Variables|Default|GetSKM_Oeil_Gr1_SKM_cils_haut_2_Gr1) (Transformation|GetActorScale3D)))