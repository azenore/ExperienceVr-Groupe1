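; BP_Son is a sound player actor that plays a given sound through its Audio component and later fades it out.
; PlaySound resets the volume multiplier, assigns and stores the sound, starts playback and prints the sound's name on screen for debugging.
; StopSound runs a timeline that drives the volume multiplier, then stops the audio and destroys the actor, so it is single-use once stopped.
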(event Custom|Stop%20Sound
  (bind _sound (Timeline|timelineson PlayFromStart)
    (:Update
      (Audio|Components|Audio|SetVolumeMultiplier (Variables|Default|GetAudio) _sound :!class /Script/Engine.AudioComponent))
    (:Finished
      (Audio|Components|Audio|Stop (Variables|Default|GetAudio))
      (Actor|DestroyActor))))

(event Custom|Play%20Sound
  (params (Sound :type Sound%20Cue%20Object%20Reference))
  (bind _audio (Variables|Default|GetAudio))
  (Audio|Components|Audio|SetVolumeMultiplier (Variables|Default|GetAudio) 1.0 :!class /Script/Engine.AudioComponent)
  (bind _output_get (Variables|Default|SetSound Sound))
  (Audio|Components|Audio|SetSound _audio _output_get)
  (Audio|Components|Audio|Play _audio 0.0)
  (Development|PrintString (Utilities|GetDisplayName (Variables|/Script/Engine.AudioComponent|GetSound _audio)) true true "(R=1.000000,G=0.030499,B=0.000000,A=1.000000)" 51.0))

(fn ConstructionScript)