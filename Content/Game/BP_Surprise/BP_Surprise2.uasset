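; BP_Surprise2 is a grabbable surprise object that bursts into a petal effect when it hits something after being dropped.
; It plays a pop sound on spawn and a magical interface cue when its GrabComponent is grabbed.
; Dropping sets a HasDropped flag, which gates the Sphere hit event that spawns the Niagara petals, calls a 2D sound and destroys the actor.
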(event OnGrabbed(GrabComponent)
  (Audio|PlaySound2D "/Game/Interface_Item_Sounds_LITE/Interface/cue/Magical_Interface_1_1_Cue.Magical_Interface_1_1_Cue" 1.0 1.0 0.0 0 0))

(event OnDropped(GrabComponent)
  (Variables|Default|SetHasDropped true))

(event OnComponentHit(Sphere)
  (params (HitComponent :type Primitive%20Component%20Object%20Reference) (OtherActor :type Actor%20Object%20Reference) (OtherComp :type Primitive%20Component%20Object%20Reference) (NormalImpulse :type Vector :default "0, 0, 0") (Hit :type Hit%20Result%20Structure%20%28by%20ref%29))
  (if (Variables|Default|GetHasDropped)
    (Niagara|SpawnSystematLocation "/Game/Game/FX/Petales/N_Petales2.N_Petales2" (Transformation|GetWorldLocation (Variables|Default|GetSphere)))
    (Audio|PlaySound2D 0 1.0 1.0 0.0 0 0)
    (Actor|DestroyActor)))

(event EventBeginPlay
  (Audio|PlaySound2D "/Game/Game/Song/SoundEffects/S_Pops.S_Pops" 1.0 1.0 0.0 0 0))

(event Collision|EventActorBeginOverlap
  (params (OtherActor :type Actor%20Object%20Reference)))

(event EventTick
  (params (DeltaSeconds :type Float%20%28single-precision%29)))

(fn ConstructionScript)