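; BPC_ComeBack is a scene component that returns its parent component to its starting place whenever it is not being held.
; On BeginPlay it stores the parent's world location and rotation and finds a GrabComponent among the parent's direct children.
; Each Tick, while that GrabComponent is not held, it lerps the parent toward the stored transform with a delta-time-scaled alpha, giving an eased return.
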(event EventBeginPlay
  (bind _returnvalue (Transformation|GetAttachParent))
  (Utilities|FlowControl|Sequence
    (:then_0
      (Variables|Default|SetTargetLocation (Transformation|GetWorldLocation _returnvalue))
      (Variables|Default|SetTargetRotation (Transformation|GetWorldRotation _returnvalue)))
    (:then_1
      (for _array_element (Components|GetChildrenComponents _returnvalue false)
        (bind _asgrab_component (Utilities|Casting|CastToGrabComponent _array_element))
        (Variables|Default|SetGrabComponent _asgrab_component)))))

(event EventTick
  (params (DeltaSeconds :type Float%20%28single-precision%29))
  (bind _returnvalue (Transformation|GetAttachParent))
  (bind _returnvalue_2 (* DeltaSeconds 5.0))
  (if (not (Variables|/Game/VRTemplate/Blueprints/GrabComponent.GrabComponent_C|GetbIsHeld (Variables|Default|GetGrabComponent)))
    (Transformation|SetWorldLocationAndRotation (Transformation|GetAttachParent) (Math|Vector|Lerp(Vector) (Transformation|GetWorldLocation _returnvalue) (Variables|Default|GetTargetLocation) _returnvalue_2) (Math|Rotator|Lerp(Rotator) (Transformation|GetWorldRotation _returnvalue) (Variables|Default|GetTargetRotation) _returnvalue_2) false false)))