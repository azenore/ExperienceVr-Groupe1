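; BP_Flar is the Flar actor, which travels along a spline in a VR game while a plane on it faces the player's camera.
; Each Tick, while IsMoving and the game has not ended, it places its sphere by elapsed time and speed, looping at the spline's length.
; That same tick fires two shine sounds; without a valid spline, it looks up a BP_Spline after a delay.
; The Deplacement function is empty.
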(event EventBeginPlay
  ;[1 1 1] Récupère et crée une variable pour la game instance et le joueur
  (bind _asbp_game_instance (Utilities|Casting|CastToBp_GameInstance (Game|GetGameInstance)))
  (Variables|Default|SetGameInstance _asbp_game_instance)
  (bind _asvrpawn (Utilities|Casting|CastToVRPawn (Game|Player|GetPlayerPawn 0)))
  (Variables|Default|SetPlayer _asvrpawn))

(event EventTick
  (params (DeltaSeconds :type Float%20%28single-precision%29))
  ;[1 1 1] Code déplacement de FLAR
  (Utilities|FlowControl|Sequence
    (:then_0
      (if (not (Variables|/Game/Game/BLUEPRINTS/Bp_GameInstance.Bp_GameInstance_C|GetTheEnd (Variables|Default|GetGameInstance)))
        (if (Variables|Default|GetIsMoving)
          (bind _bp_spline (Variables|Default|GetBP_Spline)
            (:then
              (Transformation|SetWorldLocation (Variables|Default|GetSphere) (Spline|GetLocationatDistanceAlongSpline (Variables|/Game/Game/FlarCode/BP_Spline.BP_Spline_C|GetSpline _bp_spline) (Math|Float|%(Float) (* (- (Utilities|Time|GetTimeSeconds) (Variables|Default|GetConteurTemps)) (Variables|Default|GetSpeed)) (Spline|GetSplineLength (Variables|/Game/Game/FlarCode/BP_Spline.BP_Spline_C|GetSpline _bp_spline))) "World") false false)
              (Audio|PlaySound2D "/Game/Game/Sound/SoundEffects/shine-1-268902_Cue.shine-1-268902_Cue" 1.0 1.0 0.0 0 0)
              (Audio|PlaySound2D "/Game/Game/Sound/SoundEffects/shimmering-object-79354_Cue.shimmering-object-79354_Cue" 1.0 1.0 0.0 0 0))
            (:else
              (Utilities|FlowControl|Delay 1.0)
              (Variables|Default|GetBP_Spline
                (:then)
                (:else
                  (bind _returnvalue (Actor|GetActorOfClass "/Game/Game/FlarCode/BP_Spline.BP_Spline_C"))
                  (Variables|Default|SetBP_Spline _returnvalue))))))))
    (:then_1
      (Transformation|SetWorldRotation (Variables|Default|GetPlane) (Math|Rotator|MakeRotfromZX (- (Transformation|GetWorldLocation (Variables|/Game/VRTemplate/Blueprints/VRPawn.VRPawn_C|GetCamera (Variables|Default|GetPlayer))) (Transformation|GetWorldLocation (Variables|Default|GetSphere))) (Math|Vector|MakeVector 0.0 0.0 1.0)) false false))))

(fn ConstructionScript)

(fn Deplacement)