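; BP_PinWheel is a pinwheel prop that bursts confetti when it appears and spins in response to motion.
; On BeginPlay it spawns a Niagara confetti system at its location and destroys it after a short delay.
; Each Tick adds roll to the wheel mesh, scaled by the velocity calculator component's average velocity projected onto the base mesh's right vector.
; The spin has no delta-time scaling, so its speed depends on frame rate.
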(event EventBeginPlay
  ;[1 1 1] Fait apparître des conffeti quad le moulin vent apparaît
  (bind _returnvalue (Niagara|SpawnSystematLocation "/Game/Game/FX/Confetti/NE_Confetti_System.NE_Confetti_System" (Transformation|GetActorLocation)))
  (Utilities|FlowControl|Delay 2.0)
  (Components|DestroyComponent _returnvalue))

(event EventTick
  (params (DeltaSeconds :type Float%20%28single-precision%29))
  (bind _staticmesh1 (Variables|Default|GetStaticMesh1))
  (bind _relativerotation (Variables|/Script/Engine.SceneComponent|GetRelativeRotation _staticmesh1))
  ;[1 1 1] Fait tourner le moulin a vent en fonction de la rotation du joueur
  (Transformation|SetRelativeRotation (Variables|Default|GetStaticMesh1) (Math|Rotator|MakeRotator (+ (.roll _relativerotation) (* (Math|Vector|DotProduct (Math|Vector|GetRightVector (Variables|Default|GetStaticMesh)) (Variables|/Game/Game/BLUEPRINTS/BPC/BPC_VelocityCalculator.BPC_VelocityCalculator_C|GetAverageVelocity (Variables|Default|GetBPC_VelocityCalculator))) 0.1)) (.pitch _relativerotation) (.yaw _relativerotation)) false false))

(fn ConstructionScript)