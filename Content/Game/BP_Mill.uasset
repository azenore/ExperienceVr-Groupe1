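; BP_Mill is a mill actor whose StaticMesh1 rotates in response to motion.
; Each tick it adds roll in proportion to the velocity calculator component's average velocity projected onto StaticMesh's right vector, without delta-time scaling.
; On BeginPlay it also spawns a firework Niagara effect at its location and destroys it after a short delay.
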(event EventBeginPlay
  (bind _returnvalue (Niagara|SpawnSystematLocation "/Game/Game/FX/Fireworks/FX_Firework.FX_Firework" (Transformation|GetActorLocation)))
  (Utilities|FlowControl|Delay 2.0)
  (Components|DestroyComponent _returnvalue))

(event Collision|EventActorBeginOverlap
  (params (OtherActor :type Actor%20Object%20Reference)))

(event EventTick
  (params (DeltaSeconds :type Float%20%28single-precision%29))
  (bind _staticmesh1 (Variables|Default|GetStaticMesh1))
  (bind _relativerotation (Variables|/Script/Engine.SceneComponent|GetRelativeRotation _staticmesh1))
  (Transformation|SetRelativeRotation (Variables|Default|GetStaticMesh1) (Math|Rotator|MakeRotator (+ (.roll _relativerotation) (* (Math|Vector|DotProduct (Math|Vector|GetRightVector (Variables|Default|GetStaticMesh)) (Variables|/Game/Game/BLUEPRINTS/BPC/BPC_VelocityCalculator.BPC_VelocityCalculator_C|GetAverageVelocity (Variables|Default|GetBPC_VelocityCalculator))) 0.1)) (.pitch _relativerotation) (.yaw _relativerotation)) false false))

(fn ConstructionScript)